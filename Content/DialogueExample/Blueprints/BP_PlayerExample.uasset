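; Example player character for the dialogue system demo, with hard-wired key and mouse controls to avoid project input mappings.
; Interact keys line-trace for a BPI_DialogueCore actor and pass its component to the player's dialogue handler.
; Interface events toggle the widget and input mode, while Tick requests dialogue end beyond range.
; Response identifiers trigger example events: a hard-coded wall recolor, or DT_DialogueEvents rows that spawn meshes or resize Niagara sprites.
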(event EventBPIHandleDialogueEndedResponse
  (params (Dialogue%20Widget :type User%20Widget%20Object%20Reference))
  (bind _returnvalue (Pawn|GetController))
  (bind _asplayer_controller (Utilities|Casting|CastToPlayerController _returnvalue))
  ;[1 0 0.8669] Player related events once the widget has been built and ready to be displayed and interacted with
  (Variables|Default|SetDialogueActive false)
  (Variables|Default|SetDialogue%20Actor 0)
  (Input|SetInputModeGameOnly _asplayer_controller)
  (Variables|/Script/Engine.PlayerController|SetbShowMouseCursor _asplayer_controller false)
  (Widget|RemovefromParent Dialogue%20Widget))

(event EventBPIHandleResponseIdentifier
  (params (Response%20Identifier :type Name :default "None"))
  (bind _array (Utilities|Array|MakeArray "Red" "Green" "White"))
  (bind _outitem (Utilities|Array|Random _array))
  ;[1 0.053 0] Main form of communicating unique dialogue choices externally for event executions. Once a dialogue option is selected and sends its Response Identifier from the widget to the players Dialogue Handler Component, it can then be sent elsewhere during gameplay, in the case of this example (and the default target inside of the component) the owning player character is sent the the Identifier, other places that may be benificial to send to would be your projects global event handler, or the GameMode, GameState, or even GameInstance, an example of how this could be done can be found in the Event Triggers structure attached to all dialogue choices (Check out the W_DialogueSheet_Example & AC_DialogueHandler)
  ;[1 1 1] Very Quick Examples of a player's Response Identifier Event executing some action after being received
  ;;[1 0.9648 0] Example of an event received through dialogue, potentially other ways to implement events could be through an event data table, a small example can be found right below this
  (if (== Response%20Identifier "ChangeWallColor")
    (Development|PrintString "Attempting Wall Color Change" true true "(R=1.000000,G=0.782916,B=0.000000,A=1.000000)" 3.0)
    (bind _outactors (Actor|GetAllActorswithTag "Event_WallExample"))
    (for _array_element _outactors
      (bind _asstatic_mesh_actor (Utilities|Casting|CastToStaticMeshActor _array_element))
      (if (Utilities|Array|ContainsItem (Variables|/Script/Engine.Actor|GetTags _asstatic_mesh_actor) _outitem) :!label _label
        (Utilities|FlowControl|Delay 0.01)
        (goto _label)
        (else
          (switch name _outitem
            (:Red
              (Utilities|Array|Add (Variables|/Script/Engine.Actor|GetTags _asstatic_mesh_actor) "Red")
              (Rendering|Material|SetMaterial (Variables|/Script/Engine.StaticMeshActor|GetStaticMeshComponent _asstatic_mesh_actor) 0 "/Engine/MapTemplates/Materials/BasicAsset01.BasicAsset01")
              (Utilities|Array|RemoveItem (Variables|/Script/Engine.Actor|GetTags _asstatic_mesh_actor) "Green")
              (Utilities|Array|RemoveItem (Variables|/Script/Engine.Actor|GetTags _asstatic_mesh_actor) "White"))
            (:Green
              (Utilities|Array|Add (Variables|/Script/Engine.Actor|GetTags _asstatic_mesh_actor) "Green")
              (Rendering|Material|SetMaterial (Variables|/Script/Engine.StaticMeshActor|GetStaticMeshComponent _asstatic_mesh_actor) 0 "/Engine/MapTemplates/Materials/BasicAsset03.BasicAsset03")
              (Utilities|Array|RemoveItem (Variables|/Script/Engine.Actor|GetTags _asstatic_mesh_actor) "Red")
              (Utilities|Array|RemoveItem (Variables|/Script/Engine.Actor|GetTags _asstatic_mesh_actor) "White"))
            (:White
              (Utilities|Array|Add (Variables|/Script/Engine.Actor|GetTags _asstatic_mesh_actor) "White")
              (Rendering|Material|SetMaterial (Variables|/Script/Engine.StaticMeshActor|GetStaticMeshComponent _asstatic_mesh_actor) 0 "/Engine/MapTemplates/Materials/BasicAsset02.BasicAsset02")
              (Utilities|Array|RemoveItem (Variables|/Script/Engine.Actor|GetTags _asstatic_mesh_actor) "Red")
              (Utilities|Array|RemoveItem (Variables|/Script/Engine.Actor|GetTags _asstatic_mesh_actor) "Green")))
          (Development|PrintString "Wall Color Change Successful" true true "(R=0.064483,G=1.000000,B=0.000000,A=1.000000)" 3.0))))
    (else
      ;;[0 0.3695 1] Example of a data table used to get information on how to utilize a response identifier, in this case we are spawning static meshes at a location at random, or changing the size of specifically 'tagged' particles in the level
      (bind _returnvalue (Utilities|GetDataTableRow "/Game/DialogueExample/DT/Events/DT_DialogueEvents.DT_DialogueEvents" Response%20Identifier)
        (:then
          (Development|PrintString (.StringText (Utilities|Struct|BreakS_DialogueEvent _returnvalue)) true true "(R=1.000000,G=0.782916,B=0.000000,A=1.000000)" 3.0)
          (if (not (.ChangeParticleSize (Utilities|Struct|BreakS_DialogueEvent _returnvalue)))
            (if (!= (.AddedTag (Utilities|Struct|BreakS_DialogueEvent _returnvalue)) "")
              (bind _outactors_2 (Actor|GetAllActorswithTag (.AddedTag (Utilities|Struct|BreakS_DialogueEvent _returnvalue))))
              (for _array_element_2 _outactors_2
                (Actor|DestroyActor _array_element_2))
              (for _index (range 0 (.SpawnAmount (Utilities|Struct|BreakS_DialogueEvent _returnvalue)))
                (bind _returnvalue_2 (Game|SpawnActorfromClass "/Script/Engine.StaticMeshActor" (Math|Transform|MakeTransform (- (.WorldLocation (Utilities|Struct|BreakS_DialogueEvent _returnvalue)) (Math|Vector|MakeVector (Math|Random|RandomFloatinRange (* (.WorldLocationSpread (Utilities|Struct|BreakS_DialogueEvent _returnvalue)) -1.0) (.WorldLocationSpread (Utilities|Struct|BreakS_DialogueEvent _returnvalue))) (Math|Random|RandomFloatinRange (* (.WorldLocationSpread (Utilities|Struct|BreakS_DialogueEvent _returnvalue)) -1.0) (.WorldLocationSpread (Utilities|Struct|BreakS_DialogueEvent _returnvalue))) (Math|Random|RandomFloatinRange (* (.WorldLocationSpread (Utilities|Struct|BreakS_DialogueEvent _returnvalue)) -1.0) (.WorldLocationSpread (Utilities|Struct|BreakS_DialogueEvent _returnvalue))))) (Math|Random|RandomRotator true) "1.000000,1.000000,1.000000") "Undefined" 0 0))
                (Variables|/Script/Engine.Actor|SetTags _returnvalue_2 (Utilities|Array|MakeArray (.AddedTag (Utilities|Struct|BreakS_DialogueEvent _returnvalue))))
                (Transformation|SetMobility _returnvalue_2 "Movable")
                (Components|StaticMesh|SetStaticMesh (Variables|/Script/Engine.StaticMeshActor|GetStaticMeshComponent _returnvalue_2) (.StaticMesh (Utilities|Struct|BreakS_DialogueEvent _returnvalue)))
                (if (.EnablePhysics? (Utilities|Struct|BreakS_DialogueEvent _returnvalue))
                  (Physics|SetSimulatePhysics (Variables|/Script/Engine.StaticMeshActor|GetStaticMeshComponent _returnvalue_2) true)
                  (Physics|SetEnableGravity (Variables|/Script/Engine.StaticMeshActor|GetStaticMeshComponent _returnvalue_2) true))))
            (elif (!= (.ParticleTag (Utilities|Struct|BreakS_DialogueEvent _returnvalue)) "")
              (bind _outactors_3 (Actor|GetAllActorswithTag (.ParticleTag (Utilities|Struct|BreakS_DialogueEvent _returnvalue))))
              (for _array_element_3 _outactors_3
                (bind _asniagara_actor (Utilities|Casting|CastToNiagaraActor _array_element_3))
                (Effects|Components|ParticleSystem|SetFloatParameter (Variables|/Script/Niagara.NiagaraActor|GetNiagaraComponent _asniagara_actor) "Uniform Sprite Size" (Math|Float|SelectFloat (Math|Random|RandomFloatinRange 25.0 2.5e+02) (.ParticleSize (Utilities|Struct|BreakS_DialogueEvent _returnvalue)) (< (.ParticleSize (Utilities|Struct|BreakS_DialogueEvent _returnvalue)) 0.0)))))))))))

(event EventTick
  (params (DeltaSeconds :type Float%20%28single-precision%29))
  (bind _returnvalue (Utilities|ControlRotator))
  (bind _returnvalue_2 (Math|Vector|GetRightVector _returnvalue))
  (bind _returnvalue_3 (Math|Vector|GetForwardVector _returnvalue))
  ;[1 0.05961 0] Example on how to end an active dialogue abruptly outside of dialogue itself
  (CallFunction|CheckDistancetoDialogueActor)
  ;[1 1 1] Simple Demo Controls w/o Project Inputs For Ease Of Migration
  ;;[1 1 1] Move
  (Utilities|FlowControl|Sequence
    (:then_0
      (Utilities|FlowControl|Gate true
        (:Exit
          (Pawn|Input|AddMovementInput _returnvalue_3 1.0 false))))
    (:then_1
      (Utilities|FlowControl|Gate true
        (:Exit
          (Pawn|Input|AddMovementInput _returnvalue_3 -1.0 false))))
    (:then_2
      (Utilities|FlowControl|Gate true
        (:Exit
          (Pawn|Input|AddMovementInput _returnvalue_2 -1.0 false))))
    (:then_3
      (Utilities|FlowControl|Gate true
        (:Exit
          (Pawn|Input|AddMovementInput _returnvalue_2 1.0 false))))))

(event EventBPIHandleDialogueStartedResponse
  (params (Dialogue%20Widget :type User%20Widget%20Object%20Reference) (Dialogue%20Actor :type Actor%20Object%20Reference))
  (bind _returnvalue (Pawn|GetController))
  (bind _asplayer_controller (Utilities|Casting|CastToPlayerController _returnvalue))
  ;[1 0 0.8669] Player related events once the widget has been built and ready to be displayed and interacted with
  (Variables|Default|SetDialogueActive true)
  (Variables|Default|SetDialogue%20Actor Dialogue%20Actor)
  (Input|SetInputModeGameandUI _asplayer_controller Dialogue%20Widget "DoNotLock" true)
  (Variables|/Script/Engine.PlayerController|SetbShowMouseCursor _asplayer_controller true)
  (UserInterface|Viewport|AddtoViewport Dialogue%20Widget 1))

(event Input|MouseEvents|MouseX
  (params (AxisValue :type Float%20%28single-precision%29))
  ;[1 1 1] Simple Demo Controls w/o Project Inputs For Ease Of Migration
  ;;[1 1 1] Aim
  (if (not (Variables|Default|GetDialogueActive))
    (Pawn|Input|AddControllerYawInput AxisValue)))

(event Input|MouseEvents|MouseY
  (params (AxisValue :type Float%20%28single-precision%29))
  ;[1 1 1] Simple Demo Controls w/o Project Inputs For Ease Of Migration
  ;;[1 1 1] Aim
  (if (not (Variables|Default|GetDialogueActive))
    (Pawn|Input|AddControllerPitchInput (* AxisValue -1.0))))

(event Input|KeyboardEvents|S
  (params (Key :type Key%20Structure :default "None"))
  ;[1 1 1] Simple Demo Controls w/o Project Inputs For Ease Of Migration
  ;;[1 1 1] Move
  (:Pressed
    (Utilities|FlowControl|Gate true) ; enters at Open
  )
  (:Released
    (Utilities|FlowControl|Gate true) ; enters at Close
  ))

(event Input|KeyboardEvents|W
  (params (Key :type Key%20Structure :default "None"))
  ;[1 1 1] Simple Demo Controls w/o Project Inputs For Ease Of Migration
  ;;[1 1 1] Move
  (:Pressed
    (Utilities|FlowControl|Gate true) ; enters at Open
  )
  (:Released
    (Utilities|FlowControl|Gate true) ; enters at Close
  ))

(event Input|KeyboardEvents|E
  (params (Key :type Key%20Structure :default "None"))
  ;[1 1 1] Simple Demo Controls w/o Project Inputs For Ease Of Migration
  ;;[1 1 1] Attempt to interact with a forward facing actor that has a dialogue handler
  (:Pressed
    (if (not (Default|IsInteractedHandlerValid (Variables|Default|GetAC_DialogueHandler)))
      (bind _hitactor (CallFunction|TracetoFindDialogueActor))
      (Utilities|IsValid _hitactor
        (:Is%20Valid
          (bind _dialogue_handler (Class|BPIDialogueCore|BPIGetDialogueComponent(Message) _hitactor))
          (Class|BPIDialogueCore|BPISetInteractedComponent(Message) (Variables|Default|GetAC_DialogueHandler) _dialogue_handler))))))

(event Input|KeyboardEvents|A
  (params (Key :type Key%20Structure :default "None"))
  ;[1 1 1] Simple Demo Controls w/o Project Inputs For Ease Of Migration
  ;;[1 1 1] Move
  (:Pressed
    (Utilities|FlowControl|Gate true) ; enters at Open
  )
  (:Released
    (Utilities|FlowControl|Gate true) ; enters at Close
  ))

(event Input|KeyboardEvents|D
  (params (Key :type Key%20Structure :default "None"))
  ;[1 1 1] Simple Demo Controls w/o Project Inputs For Ease Of Migration
  ;;[1 1 1] Move
  (:Pressed
    (Utilities|FlowControl|Gate true) ; enters at Open
  )
  (:Released
    (Utilities|FlowControl|Gate true) ; enters at Close
  ))

(event Input|MouseEvents|LeftMouseButton
  (params (Key :type Key%20Structure :default "None"))
  ;[1 1 1] Simple Demo Controls w/o Project Inputs For Ease Of Migration
  ;;[1 1 1] Attempt to interact with a forward facing actor that has a dialogue handler
  (:Pressed
    (if (not (Default|IsInteractedHandlerValid (Variables|Default|GetAC_DialogueHandler)))
      (bind _hitactor (CallFunction|TracetoFindDialogueActor))
      (Utilities|IsValid _hitactor
        (:Is%20Valid
          (bind _dialogue_handler (Class|BPIDialogueCore|BPIGetDialogueComponent(Message) _hitactor))
          (Class|BPIDialogueCore|BPISetInteractedComponent(Message) (Variables|Default|GetAC_DialogueHandler) _dialogue_handler))))))

(event Input|MouseEvents|RightMouseButton
  (params (Key :type Key%20Structure :default "None"))
  ;[1 1 1] Simple Demo Controls w/o Project Inputs For Ease Of Migration
  ;;[1 1 1] Attempt to interact with a forward facing actor that has a dialogue handler
  (:Pressed
    (if (not (Default|IsInteractedHandlerValid (Variables|Default|GetAC_DialogueHandler)))
      (bind _hitactor (CallFunction|TracetoFindDialogueActor))
      (Utilities|IsValid _hitactor
        (:Is%20Valid
          (bind _dialogue_handler (Class|BPIDialogueCore|BPIGetDialogueComponent(Message) _hitactor))
          (Class|BPIDialogueCore|BPISetInteractedComponent(Message) (Variables|Default|GetAC_DialogueHandler) _dialogue_handler))))))

(event Input|KeyboardEvents|F
  (params (Key :type Key%20Structure :default "None"))
  ;[1 1 1] Simple Demo Controls w/o Project Inputs For Ease Of Migration
  ;;[1 1 1] Attempt to interact with a forward facing actor that has a dialogue handler
  (:Pressed
    (if (not (Default|IsInteractedHandlerValid (Variables|Default|GetAC_DialogueHandler)))
      (bind _hitactor (CallFunction|TracetoFindDialogueActor))
      (Utilities|IsValid _hitactor
        (:Is%20Valid
          (bind _dialogue_handler (Class|BPIDialogueCore|BPIGetDialogueComponent(Message) _hitactor))
          (Class|BPIDialogueCore|BPISetInteractedComponent(Message) (Variables|Default|GetAC_DialogueHandler) _dialogue_handler))))))

(event Input|KeyboardEvents|R
  (params (Key :type Key%20Structure :default "None"))
  ;[1 1 1] Simple Demo Controls w/o Project Inputs For Ease Of Migration
  ;;[1 1 1] Attempt to interact with a forward facing actor that has a dialogue handler
  (:Pressed
    (if (not (Default|IsInteractedHandlerValid (Variables|Default|GetAC_DialogueHandler)))
      (bind _hitactor (CallFunction|TracetoFindDialogueActor))
      (Utilities|IsValid _hitactor
        (:Is%20Valid
          (bind _dialogue_handler (Class|BPIDialogueCore|BPIGetDialogueComponent(Message) _hitactor))
          (Class|BPIDialogueCore|BPISetInteractedComponent(Message) (Variables|Default|GetAC_DialogueHandler) _dialogue_handler))))))

(fn ConstructionScript)

(fn TracetoFindDialogueActor
  (bind _returnvalue (Transformation|GetActorLocation))
  (bind (_outhit _returnvalue_2) (Collision|LineTraceByChannel _returnvalue (+ _returnvalue (* (Transformation|GetActorForwardVector) 5e+02)) "TraceTypeQuery1" false (Utilities|Array|MakeArray self) "ForDuration" true "(R=1.000000,G=0.000000,B=0.000000,A=1.000000)" "(R=0.000000,G=1.000000,B=0.000000,A=1.000000)" 2.0))
  (if _returnvalue_2
    (if (Utilities|DoesObjectImplementInterface (.HitActor (Collision|BreakHitResult _outhit)) "/Game/DialogueCore/Interface/BPI_DialogueCore.BPI_DialogueCore_C")
      (return (.HitActor (Collision|BreakHitResult _outhit)))
      (else
        _)))
  (return 0))

(fn CheckDistancetoDialogueActor
  (bind _dialogue_actor (Variables|Default|GetDialogue%20Actor))
  (Utilities|IsValid _dialogue_actor
    (:Is%20Valid
      (if (> (Transformation|GetDistanceTo _dialogue_actor) 3e+02)
        ;[1 0 0.5983] Using this interface function targetted at a player's dialogue handler will attempt to 'cleanly' end any active conversation
        (Class|BPIDialogueCore|BPIAttemptEndActiveDialogue(Message) (Variables|Default|GetAC_DialogueHandler))
        (return)
        (else
          (return))))
    (:Is%20Not%20Valid
      (return))))

(fn BPIGetDialogueComponent
  (return (Variables|Default|GetAC_DialogueHandler)))

(fn BPIGetDialogueSpeakerName
  (return (Variables|/Game/DialogueCore/Components/AC_DialogueHandler.AC_DialogueHandler_C|GetSpeaker%20Name (Variables|Default|GetAC_DialogueHandler))))