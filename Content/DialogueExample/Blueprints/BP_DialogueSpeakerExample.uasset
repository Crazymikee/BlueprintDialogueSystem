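; BP_DialogueSpeakerExample is an example NPC dialogue speaker that players can converse with.
; On BeginPlay it passes an example dialogue data table and speaker name to its dialogue handler component, overriding the defaults.
; Interface functions expose that component and the speaker name.
; An interface event sent from the interacting player's widget plays a montage on the NPC's skeletal mesh.
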(event EventBeginPlay
  (bind _ac_dialoguehandler (Variables|Default|GetAC_DialogueHandler))
  ;[1 0 0.1259] Override default Dialogue Handler values for conversation + name
  (Class|BPIDialogueCore|BPIHandleInitialDialogueData(Message) _ac_dialoguehandler (Variables|Default|GetDialogue%20DT%20Example))
  (Class|BPIDialogueCore|BPISetDialogueSpeakerName(Message) _ac_dialoguehandler "Cube Man"))

(event EventBPISendSpeakerMontage
  (params (Montage :type Anim%20Montage%20Object%20Reference))
  ;[1 0.9426 0] Event sent from the interacted players widget, useful for playing a montage on the host npcs skeletal mesh, among other things that could be expanded upon for your project
  (Animation|Montage|PlayMontage (Variables|Default|GetSkeletalMesh) Montage))

(fn ConstructionScript)

(fn BPIGetDialogueComponent
  (return (Variables|Default|GetAC_DialogueHandler)))

(fn BPIGetDialogueSpeakerName
  (return (Variables|/Game/DialogueCore/Components/AC_DialogueHandler.AC_DialogueHandler_C|GetSpeaker%20Name (Variables|Default|GetAC_DialogueHandler))))