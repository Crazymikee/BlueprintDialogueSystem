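; Dialogue component for both player pawns and the speakers they talk to.
; Speaker side merges DataTable conversations and added responses into CoreDialogueBody, baking "Initially Random" lines into fixed rows.
; Player side creates the dialogue widget, feeds it the interacted handler's body, and relays start, end and response identifiers to its owner through interface messages.
; An alternative response event can target the owner, GameMode, GameState or GameInstance.
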(event Custom|Initialize
  ;[1 0 0.9362] Initialize Player Widget (Make sure this is only allowed to happen on player controlled characters)
  (if (Variables|DialogueSettings|Player|GetPlayerOwned)
    (bind _aspawn (Utilities|Casting|CastToPawn (Components|GetOwner))
      (:then
        (bind _asplayer_controller (Utilities|Casting|CastToPlayerController (Pawn|GetController _aspawn))
          (:then
            (bind _returnvalue (UserInterface|CreateWidget (Variables|DialogueSettings|Player|GetPlayerWidgetClass) _asplayer_controller))
            (bind _output_get (Variables|Core|SetDialogueWidget _returnvalue))
            (Utilities|IsValid _output_get
              (:Is%20Valid
                (Class|BPIDialogueCore|BPISetDialogueComponent(Message) _output_get self))
              (:Is%20Not%20Valid
                (Development|PrintString "Error: Dialogue Handler failed to create player widget" true true "(R=1.000000,G=0.000000,B=0.000000,A=1.000000)" 5.0))))
          (:CastFailed
            (Development|PrintString "Error: Dialogue Handler is NOT able to find a valid player controller" true true "(R=1.000000,G=0.000000,B=0.000000,A=1.000000)" 5.0))))
      (:CastFailed
        (Development|PrintString "Error: Dialogue Handler is NOT on a valid pawn" true true "(R=1.000000,G=0.000000,B=0.000000,A=1.000000)" 5.0)))))

(event EventBeginPlay
  ;[0 0.4056 1] Begin Play
  (CallFunction|Initialize))

(event EventBPISetDialogueSpeakerName
  (params (Speaker%20Name :type Text))
  ;[1 0.848 0] Universal: Handler name in dialogue
  (Variables|DialogueSettings|Universal|SetSpeaker%20Name Speaker%20Name))

(event EventBPIHandleInitialDialogueData
  (params (Dialogue%20Initial%20Data :type S%20Dialogue%20Initial%20Data%20Structure))
  ;[0 1 0] Non-Player: Initial Dialogue Body Creation
  (Core|BuildInitialDialogueData Dialogue%20Initial%20Data))

(event EventBPIHandleDialogueEndedResponse
  (params (Dialogue%20Widget :type User%20Widget%20Object%20Reference))
  ;[1 0.7569 0] Player: End dialogue with an interacted handler, either through dialogue or externally, removing the interacted dialogue handler reference and notifying the player actor to resume previous state, in most cases disabling/hiding cursor and allowing aiming/movement among other things specific to different games
  (Utilities|IsValid (Variables|Core|GetInteracted%20Handler)
    (:Is%20Valid
      (Variables|Core|SetInteracted%20Handler 0))
    (:Is%20Not%20Valid
      _))
  (Class|BPIDialogueCore|BPIHandleDialogueEndedResponse(Message) (Components|GetOwner) (Variables|Core|GetDialogueWidget)))

(event EventBPISetInteractedComponent
  (params (Interacted%20Handler :type AC%20Dialogue%20Handler%20Object%20Reference))
  ;[0 0.7074 1] Player: Start dialogue with an interacted handler, sending events to the widget to display the conversation, and to the player to do various tasks like unlock mouse ui mode, display mouse, and whatever else the player character may need to do for proper navigation of the ui widget
  (Utilities|IsValid (Variables|Core|GetInteracted%20Handler)
    (:Is%20Valid
      (Development|PrintString "Error: Dialogue Handler already has registered with another component" true true "(R=1.000000,G=0.000000,B=0.000000,A=1.000000)" 5.0))
    (:Is%20Not%20Valid
      (bind _output_get (Variables|Core|SetInteracted%20Handler Interacted%20Handler))
      (Class|BPIDialogueCore|BPIBuildDialoguetoWidget(Message) (Variables|Core|GetDialogueWidget) (Variables|AC_DialogueHandler_C|GetCoreDialogueBody _output_get) (Components|GetOwner _output_get))
      (Class|BPIDialogueCore|BPIHandleDialogueStartedResponse(Message) (Components|GetOwner) (Variables|Core|GetDialogueWidget) (Components|GetOwner _output_get)))))

(event EventBPIAttemptEndActiveDialogue
  ;[1 0.7569 0] Player: End dialogue with an interacted handler, either through dialogue or externally, removing the interacted dialogue handler reference and notifying the player actor to resume previous state, in most cases disabling/hiding cursor and allowing aiming/movement among other things specific to different games
  (Utilities|IsValid (Variables|Core|GetInteracted%20Handler)
    (:Is%20Valid
      (Variables|Core|SetInteracted%20Handler 0))
    (:Is%20Not%20Valid
      _))
  (Class|BPIDialogueCore|BPIAttemptEndActiveDialogue(Message) (Variables|Core|GetDialogueWidget)))

(event EventBPISetCurrentDialogueBody
  (params (Body%20Key :type Name :default "None"))
  ;[1 0.2756 0] Player: Set current active dialogue body, used for dynamic rebuilding
  (Variables|Core|SetBody%20Key Body%20Key))

(event EventBPIHandleResponseIdentifier
  (params (Response%20Identifier :type Name :default "None"))
  ;[1 0.01705 0] Player: Reaction to selecting an answer that hosts a Response Identifier allowing the parent actor to know about a unique dialogue choice to act upon
  (Class|BPIDialogueCore|BPIHandleResponseIdentifier(Message) (Components|GetOwner) Response%20Identifier))

(event EventBPIHandleResponseIdentifierAlternative
  (params (ResponseIdentifier :type Name :default "None") (Event%20Triggers :type S%20Dialogue%20Event%20Triggers%20Structure))
  ;[0 1 0.08014] Player: An alternative Response Identifier Event you can implement in your dialogue widget that has the Event Triggers Structure that is able to be expanded upon to add more functionality to player responses depending on your projects internal data and variable uses, in the case of this example we are using an enumeration to select a specific target object to send our Response Identifier to for event execution (See W_DialogueSheet_Example in the response selected section) Note this is not active by default
  (Class|BPIDialogueCore|BPIHandleResponseIdentifierAlternative(Message) (Utilities|Select :Index (.ResponseIdentifierTarget (Utilities|Struct|BreakS_DialogueEventTriggers Event%20Triggers)) :NewEnumerator0 (Components|GetOwner) :NewEnumerator1 (Game|GetGameMode) :NewEnumerator2 (Game|GetGameState) :NewEnumerator3 (Game|GetGameInstance)) ResponseIdentifier Event%20Triggers))

(fn BuildInitialDialogueData
  (params (Dialogue%20DT%20Info :type S%20Dialogue%20Initial%20Data%20Structure))
  (bind _localdialoguebody (LocalVariables|GetLocalDialogueBody))
  (bind _localdialoguebody_2 (LocalVariables|GetLocalDialogueBody))
  (bind _conversationbody (Utilities|Struct|BreakS_DialogueBody _localdialoguebody))
  (bind _conversationbody_2 (Utilities|Struct|BreakS_DialogueBody _localdialoguebody_2))
  (bind _output_get (Variables|DialogueSettings|NonPlayer|SetNonPlayerDialogueData Dialogue%20DT%20Info))
  (LocalVariables|SetLocalResponseAdditions (.DialogueResponseAdditions (Utilities|Struct|BreakS_DialogueInitialData _output_get)))
  ;[0.05452 1 0] Build Speaker Map
  (for _array_element (.DialogueRootData (Utilities|Struct|BreakS_DialogueInitialData _output_get))
    (bind _returnvalue (Utilities|GetDataTableRow (.DataTable (Utilities|Struct|BreakS_DataTableInfo _array_element)) (.DataTableRow (Utilities|Struct|BreakS_DataTableInfo _array_element)))
      (:then
        (bind _keys (Utilities|Map|Keys (.ConversationBody (Utilities|Struct|BreakS_DialogueRoot _returnvalue))))
        (bind _values (Utilities|Map|Values (.ConversationBody (Utilities|Struct|BreakS_DialogueRoot _returnvalue))))
        (Utilities|Array|AppendArray (LocalVariables|GetLocalResponseAdditions) (.PlayerResponseAddition (Utilities|Struct|BreakS_DialogueRoot _returnvalue)))
        (for (_array_element_2 _array_index) _keys
          (Utilities|Map|Add (Utilities|Struct|BreakS_DialogueBody (LocalVariables|GetLocalDialogueBody)) _array_element_2 (Utilities|Array|Get(acopy) _values _array_index))))))
  ;[0 0.925 1] Build Player Response Arrays
  (for _array_element_3 (LocalVariables|GetLocalResponseAdditions)
    (Utilities|Array|Clear (LocalVariables|GetLocalResponseModified))
    (if (.ReturnValue (Utilities|Map|Find _conversationbody (.ConversationKey (Utilities|Struct|BreakS_DialogueSpeakerResponseAddition _array_element_3))))
      (bind _output_get_2 (LocalVariables|SetLocalResponseModified (.PlayerResponses (Utilities|Struct|BreakS_DialogueSpeakerResponse (.Value (Utilities|Map|Find _conversationbody (.ConversationKey (Utilities|Struct|BreakS_DialogueSpeakerResponseAddition _array_element_3))))))))
      (Utilities|Array|AddUnique _output_get_2 (.AddedResponse (Utilities|Struct|BreakS_DialogueSpeakerResponseAddition _array_element_3)))
      (Utilities|Map|Add _conversationbody (.ConversationKey (Utilities|Struct|BreakS_DialogueSpeakerResponseAddition _array_element_3)) (Utilities|Struct|MakeS_DialogueSpeakerResponse (.TextData (Utilities|Struct|BreakS_DialogueSpeakerResponse (.Value (Utilities|Map|Find _conversationbody (.ConversationKey (Utilities|Struct|BreakS_DialogueSpeakerResponseAddition _array_element_3)))))) (LocalVariables|GetLocalResponseModified)))))
  ;[1 0.4217 0] Modify all Text Data searching for 'Initially Random' dialogue
  (bind _keys_2 (Utilities|Map|Keys _conversationbody_2))
  (bind _values_2 (Utilities|Map|Values _conversationbody_2))
  (for (_array_element_4 _array_index_2) _values_2
    (Utilities|Array|Clear (LocalVariables|GetLocalResponseModified))
    (switch Utilities|FlowControl|Switch|SwitchonE_DialogueTextType (.DialogueDTRowType (Utilities|Struct|BreakS_DialogueTextData (.TextData (Utilities|Struct|BreakS_DialogueSpeakerResponse _array_element_4))))
      (:NewEnumerator0
        (LocalVariables|SetLocalTextData (.TextData (Utilities|Struct|BreakS_DialogueSpeakerResponse _array_element_4)) :!label _label))
      (:NewEnumerator1
        (goto _label))
      (:NewEnumerator2
        (LocalVariables|SetLocalTextData (Utilities|Struct|MakeS_DialogueTextData "NewEnumerator0" (Utility|GetRandomDataTableRow (.DialogueDataTable (Utilities|Struct|BreakS_DialogueTextData (.TextData (Utilities|Struct|BreakS_DialogueSpeakerResponse _array_element_4))))) (.DialogueDataTable (Utilities|Struct|BreakS_DialogueTextData (.TextData (Utilities|Struct|BreakS_DialogueSpeakerResponse _array_element_4))))))))
    (for _array_element_5 (.PlayerResponses (Utilities|Struct|BreakS_DialogueSpeakerResponse _array_element_4))
      (switch Utilities|FlowControl|Switch|SwitchonE_DialogueTextType (.DialogueDTRowType (Utilities|Struct|BreakS_DialogueTextData (.TextData (Utilities|Struct|BreakS_DialoguePlayerResponse _array_element_5))))
        (:NewEnumerator0
          (Utilities|Array|AddUnique (LocalVariables|GetLocalResponseModified) _array_element_5 :!label _label_2))
        (:NewEnumerator1
          (goto _label_2))
        (:NewEnumerator2
          (Utilities|Array|AddUnique (LocalVariables|GetLocalResponseModified) (Utilities|Struct|MakeS_DialoguePlayerResponse (.ResponseType (Utilities|Struct|BreakS_DialoguePlayerResponse _array_element_5)) (.SwitchMapKey (Utilities|Struct|BreakS_DialoguePlayerResponse _array_element_5)) (.ResponseIdentifier (Utilities|Struct|BreakS_DialoguePlayerResponse _array_element_5)) (Utilities|Struct|MakeS_DialogueTextData "NewEnumerator0" (Utility|GetRandomDataTableRow (.DialogueDataTable (Utilities|Struct|BreakS_DialogueTextData (.TextData (Utilities|Struct|BreakS_DialoguePlayerResponse _array_element_5))))) (.DialogueDataTable (Utilities|Struct|BreakS_DialogueTextData (.TextData (Utilities|Struct|BreakS_DialoguePlayerResponse _array_element_5))))) (.EventTriggers (Utilities|Struct|BreakS_DialoguePlayerResponse _array_element_5)))))))
    (Utilities|Map|Add (Utilities|Struct|BreakS_DialogueBody (LocalVariables|GetLocalDialogueBody)) (Utilities|Array|Get(acopy) _keys_2 _array_index_2) (Utilities|Struct|MakeS_DialogueSpeakerResponse (LocalVariables|GetLocalTextData) (LocalVariables|GetLocalResponseModified))))
  ;;[1 0 0.8033] Finish
  (Variables|Core|SetCoreDialogueBody (LocalVariables|GetLocalDialogueBody))
  (return))

(fn GenerateDialogueText
  (params (Text%20Data :type S%20Dialogue%20Text%20Data%20Structure))
  (bind (_dialoguedtrowtype _dialoguespecificdtrow _dialoguedatatable) (Utilities|Struct|BreakS_DialogueTextData Text%20Data))
  (Utilities|IsValid _dialoguedatatable
    (:Is%20Valid
      (switch Utilities|FlowControl|Switch|SwitchonE_DialogueTextType _dialoguedtrowtype
        (:NewEnumerator0
          (bind _returnvalue (Utilities|GetDataTableRow _dialoguedatatable _dialoguespecificdtrow)
            (:then
              (return (.Text (Utilities|Struct|BreakS_DataTableText _returnvalue)) (.Audio (Utilities|Struct|BreakS_DataTableText _returnvalue)) (.SpeakerMontage (Utilities|Struct|BreakS_DataTableText _returnvalue))))
            (:RowNotFound
              _)))
        (:NewEnumerator1
          (bind _outrownames (DataTable|GetDataTableRowNames _dialoguedatatable :!label _label))
          (bind _returnvalue_2 (Utilities|GetDataTableRow _dialoguedatatable (.OutItem (Utilities|Array|Random _outrownames)))
            (:then
              (return (.Text (Utilities|Struct|BreakS_DataTableText _returnvalue_2)) (.Audio (Utilities|Struct|BreakS_DataTableText _returnvalue_2)) (.SpeakerMontage (Utilities|Struct|BreakS_DataTableText _returnvalue_2))))
            (:RowNotFound
              _)))
        (:NewEnumerator2
          (goto _label)))
      (return (Utilities|Text|ToText(Name) "Error: Table Row Not Found") 0 0))
    (:Is%20Not%20Valid
      (return (Utilities|Text|ToText(Name) _dialoguespecificdtrow) 0 0))))

(fn GetRandomDataTableRow
  (params (Table :type Data%20Table%20Object%20Reference))
  (Utilities|IsValid Table
    (:Is%20Valid
      (bind _outrownames (DataTable|GetDataTableRowNames Table))
      (return (.OutItem (Utilities|Array|Random _outrownames))))
    (:Is%20Not%20Valid
      (return "None"))))

(fn IsInteractedHandlerValid
  (return (Utilities|IsValid (Variables|Core|GetInteracted%20Handler))))

(fn BPIGetDialogueComponent
  (return 0))

(fn BPIGetDialogueSpeakerName
  (return (Variables|DialogueSettings|Universal|GetSpeaker%20Name)))